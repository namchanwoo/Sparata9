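; BP_ChatMode is a game mode for a chat-driven answer game, relaying client messages and submitting them as numeric guesses.
; BeginPlay delays StartGame briefly so all player controllers finish registering first.
; Each client message goes to the stored server controller's GotBroadcast, then to TryAnswer with the sender's ID.
; GetALLUserIDs rebuilds the joined-controller list from all BP_Controller actors; StartGame and TryAnswer are defined outside this graph.
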(event Custom|GotMessageFromClient
  (params (Msg :type String) (UserID :type String))
  (Default|GotBroadcast (Variables|Default|GetServerController) Msg)
  (Class|BaseballGameModeBase|TryAnswer UserID Msg))

(event Custom|SetServerController
  (params (ServerController :type BP%20Controller%20Object%20Reference))
  (Variables|Default|SetServerController ServerController))

(event EventBeginPlay
  ;[0.15 0.15 0.15 0.5] 딜레이 없으면 시작할 때 플레이어 컨트롤러가 다 등록되지 않음.
  (Utilities|FlowControl|Delay 2.0)
  (Class|BaseballGameModeBase|StartGame))

(event EventTick
  (params (DeltaSeconds :type Float%20%28single-precision%29)))

(event EventGetALLUserIDs
  (Utilities|Array|Clear (Variables|Default|GetJoinedUserControllers))
  (bind _outactors (Actor|GetAllActorsOfClass "/Game/Blueprints/BP_Controller.BP_Controller_C"))
  (for _array_element _outactors
    (Utilities|Array|Add (Variables|Default|GetJoinedUserControllers) _array_element)))

(fn ConstructionScript)